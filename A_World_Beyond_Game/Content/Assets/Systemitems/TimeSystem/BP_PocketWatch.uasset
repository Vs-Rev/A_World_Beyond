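; BP_PocketWatch is a pocket watch actor whose hands show the current real-world system time.
; BeginPlay deactivates the watch, minute and second hand components, then starts a one-second Delay loop instead of using Tick.
; Each pass sets the hands' relative pitch from Now(), with the hour hand advancing by minutes and the second hand scaled by SecondsTime.
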(event EventBeginPlay
  (bind _returnvalue (Math|DateTime|Now))
  (bind (_year _month _day _hour _minute _second) (Math|DateTime|BreakDateTime _returnvalue))
  (Components|Activation|SetActive (Variables|Default|GetSekundenzeiger) false false)
  (Transformation|SetRelativeRotation (Variables|Default|GetStundenzeiger) (Math|Rotator|MakeRotator 0.0 (* (+ (Math|Conversions|ToFloat(Integer) (* _hour 30)) (/ (Math|Conversions|ToFloat(Integer) _minute) 2.0)) -1.0) 0.0) false false :!label _label)
  (Transformation|SetRelativeRotation (Variables|Default|GetMinutenzeiger) (Math|Rotator|MakeRotator 0.0 (Math|Conversions|ToFloat(Integer) (* _minute -6)) 0.0) false false)
  (Transformation|SetRelativeRotation (Variables|Default|GetSekundenzeiger) (Math|Rotator|Lerp(Rotator) (Math|Rotator|MakeRotator 0.0 (Math|Conversions|ToFloat(Integer) (* _second (Variables|Default|GetSecondsTime))) 0.0) "0, 0, 0" 0.0) false false)
  (Utilities|FlowControl|Delay 1.0)
  (goto _label))

(event Collision|EventActorBeginOverlap
  (params (OtherActor :type Actor%20Object%20Reference)))

(event EventTick
  (params (DeltaSeconds :type Float%20%28single-precision%29)))

(fn ConstructionScript)